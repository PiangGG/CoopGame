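; Game mode Blueprint that spawns tracker bots at locations chosen by an environment query.
; SpawnNewBot runs EQS_FindSpawnLocation in random-best-25% mode, then on success draws a debug sphere and spawns BP_STrackBot at each returned location, adjusting for collisions.
; An actor-killed handler validates victim and killer and prints a message, but its binding and the player-state score award are disconnected, and BeginPlay is empty.
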(event `self.SpawnNewBot`
  (bind _returnvalue (`EnvQueryManager.RunEQSQuery` "/Game/Blueprints/EQS_FindSpawnLocation.EQS_FindSpawnLocation" self "RandomBest25Pct"))
  (add `EnvQueryInstanceBlueprintWrapper.OnQueryFinishedEvent` _returnvalue (delegate `OnQueryFinishedEvent_事件_0`)))

(event `OnQueryFinishedEvent_事件_0`
  (params (QueryInstance :type "EnvQueryInstanceBlueprintWrapper Object Reference") (QueryStatus :type "EEnvQueryStatus Enum" :default "Processing"))
  (switch `EEnvQueryStatus` QueryStatus
    (:`Success`
      (bind _resultlocations (`EnvQueryInstanceBlueprintWrapper.GetQueryResultsAsLocations` QueryInstance))
      (for _array_element _resultlocations
        (`KismetSystemLibrary.DrawDebugSphere` _array_element 50.0 12 (struct :`R` 1.0 :`G` 1.0 :`B` 1.0 :`A` 1.0) 2.0 2.0)
        (`|SpawnActorFromClass` "/Game/TrackBot/BP_STrackBot.BP_STrackBot_C" (`KismetMathLibrary.MakeTransform` _array_element) "AdjustIfPossibleButDontSpawnIfColliding" "OverrideRootScale" null null)))))

(event `self.ReceiveBeginPlay`)

(event `OnActorKilled_事件_0` :!signature `self.OnActorKilled`
  (params (VitActor :type "Actor Object Reference") (KillerActor :type "Actor Object Reference") (KillerController :type "Controller Object Reference"))
  (bind _returnvalue (`Controller.K2_GetPawn` KillerController))
  (bind _aspawn (cast `Pawn` VitActor))
  (if (`Pawn.IsPawnControlled` _aspawn)
    (`/Engine/EditorBlueprintResources/StandardMacros.IsValid` KillerController
      (:`Is Valid`
        (`/Engine/EditorBlueprintResources/StandardMacros.IsValid` _returnvalue
          (:`Is Valid`
            (`/Engine/EditorBlueprintResources/StandardMacros.IsValid` (`Pawn.PlayerState` _returnvalue)
              (:`Is Valid`
                (`KismetSystemLibrary.PrintString` "Hello" true true (struct :`R` 1.0 :`G` 0.254498 :`B` 0.344261 :`A` 1.0))))))))))

(fn `UserConstructionScript`)