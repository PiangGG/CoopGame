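; Character Blueprint that sets up the on-screen HUD for the local player.
; On BeginPlay it checks for a valid, local player controller, then creates the WBP_Cross and WBP_Health widgets and adds them to the viewport.
; Tick and the construction script are empty, and debug prints of walk speed and HealthComponent health are left unconnected.
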(event `self.ReceiveBeginPlay`
  (bind _returnvalue (`self.GetController`))
  (`/Engine/EditorBlueprintResources/StandardMacros.IsValid` _returnvalue
    (:`Is Valid`
      (if (`Controller.IsLocalPlayerController` _returnvalue)
        (`|ExecutionSequence`
          (:`then_0`
            (bind _returnvalue_2 (`|CreateWidget` "/Game/Blueprints/WBP_Cross.WBP_Cross_C"))
            (`UserWidget.AddToViewport` _returnvalue_2 0))
          (:`then_1`
            (bind _returnvalue_3 (`|CreateWidget` "/Game/Blueprints/WBP_Health.WBP_Health_C"))
            (`UserWidget.AddToViewport` _returnvalue_3 0)))))))

(event `self.ReceiveTick`
  (params (DeltaSeconds :type "Float (single-precision)")))

(fn `UserConstructionScript`)